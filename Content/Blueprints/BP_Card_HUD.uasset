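; HUD Blueprint for a card game that draws the remaining move count on screen.
; On BeginPlay it caches the BP_LogicMem game mode, which supplies the counter and its visibility flag.
; Each DrawHUD, when the flag is on, it projects a fixed world position to screen space and centers the white text there using its measured size.
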(event `self.ReceiveBeginPlay`
  ;[1 1 1] Cache reference to LogicMem
  (bind _asbp_logic_mem (cast `/Game/Blueprints/BP_LogicMem` (`GameplayStatics.GetGameMode`)))
  (set `self.LogicMem` _asbp_logic_mem))

(event `self.ReceiveDrawHUD`
  (params (SizeX :type Integer) (SizeY :type Integer))
  (bind _logicmem (`self.LogicMem`))
  (bind _returnvalue (`KismetStringLibrary.Conv_IntToString` (`/Game/Blueprints/BP_LogicMem.MovesCounter` _logicmem)))
  (bind (_outwidth _outheight) (`self.GetTextSize` _returnvalue "/Engine/EngineFonts/RobotoDistanceField.RobotoDistanceField" 2.0))
  ;[1 1 1] Draw moves remaining
  (if (`/Game/Blueprints/BP_LogicMem.Show move counter` _logicmem)
    (`self.DrawText` _returnvalue (struct :`R` 1.0 :`G` 1.0 :`B` 1.0 :`A` 1.0) (- (.x (`self.Project` (73.0 17.5 44.299999))) (* _outwidth 0.5)) (- (.y (`self.Project` (73.0 17.5 44.299999))) (* _outheight 0.5)) "/Engine/EngineFonts/RobotoDistanceField.RobotoDistanceField" 2.0) ; Display number of moves left
  ))

(fn `UserConstructionScript`)