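; BP_ParticleSnowBox is an actor that drives a snow particle system component, ParticleSnowBox2.
; The construction script sets the particle parameters snowScaleA and snowScaleB to zero.
; BeginPlay then sets both parameters from the SnowScaleA and SnowScaleB variables, so the configured snow scales apply only once play starts.
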(event `self.ReceiveBeginPlay`
  (`ParticleSystemComponent.SetFloatParameter` (`self.ParticleSnowBox2`) "snowScaleA" (`self.snowScaleA`))
  (`ParticleSystemComponent.SetFloatParameter` (`self.ParticleSnowBox2`) "snowScaleB" (`self.snowScaleB`)))

(event `self.ReceiveActorBeginOverlap`
  (params (OtherActor :type "Actor Object Reference")))

(fn `UserConstructionScript`
  (`ParticleSystemComponent.SetFloatParameter` (`self.ParticleSnowBox2`) "snowScaleA" 0.0)
  (`ParticleSystemComponent.SetFloatParameter` (`self.ParticleSnowBox2`) "snowScaleB" 0.0))