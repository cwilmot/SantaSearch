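; Memory-game card actor that shows an animal picture set by its type index and reports clicks or touches to BP_LogicMem unless blocked.
; Timelines move it between the Deck and its BoardIndex grid slot, and flip it with sound and particles.
; Two cross-controlled gates alternate RotateCard and UnRotateCard.
; ActivateParticleFX plays match, mismatch or black-match feedback, destroying matched cards but only hiding and disabling collision on black matches.
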(event `ActivateParticleFX`
  (params (CardsMatch :type Boolean) (BlackMatch :type Boolean))
  ;[1 1 1] ParticleEffects and sounds when comparing cards
  (set `self.BlockClick` true)
  (if CardsMatch
    (`ActorComponent.Activate` (`self.GoodMatch`) true)
    (`|ExecutionSequence`
      (:`then_0`
        (`GameplayStatics.PlaySoundAtLocation` "/Game/Assets/Sounds/Card_Match_Stereo_Cue.Card_Match_Stereo_Cue") ; Sound Card Match
      )
      (:`then_1`
        (`KismetSystemLibrary.Delay` 0.2)
        (`SceneComponent.SetVisibility` (`self.CardPicture`) false true)
        (`self.SetActorEnableCollision` false)
        (`KismetSystemLibrary.Delay` 1.2)
        (set `self.BlockClick` false)
        (`self.K2_DestroyActor`)))
    (elif BlackMatch
      (`ActorComponent.Activate` (`self.BlackMatch`) true)
      (`|ExecutionSequence`
        (:`then_0`
          (`GameplayStatics.PlaySoundAtLocation` "/Game/Assets/Sounds/Card_Mismatch_Stereo_Cue.Card_Mismatch_Stereo_Cue" :!label _label) ; Sound CardMismatch
          (`KismetSystemLibrary.Delay` 1.2)
          (set `self.BlockClick` false))
        (:`then_1`
          (`KismetSystemLibrary.Delay` 0.2)
          (`SceneComponent.SetVisibility` (`self.CardPicture`) false true)
          (`self.SetActorEnableCollision` false)))
      (else
        (`ActorComponent.Activate` (`self.BadMatch`) true)
        (goto _label)))))

(event `self.CardPicture.OnClicked`
  (params (TouchedComponent :type "PrimitiveComponent Object Reference"))
  ;[1 1 1] Card is clicked on
  (if (not (`self.BlockClick`)) :!label _label_2
    (bind _asbp_logic_mem (cast `/Game/Blueprints/BP_LogicMem` (`self.Logic`)))
    (`/Game/Blueprints/BP_LogicMem.SetClickedCard` _asbp_logic_mem self (`self.CardIType`)) ; Tell LogicMem about card being clicked
  ))

(event `self.CardPicture.OnInputTouchBegin`
  (params (FingerIndex :type "ETouchIndex Enum" :default "Touch1") (TouchedComponent :type "PrimitiveComponent Object Reference"))
  ;[1 1 1] Card is clicked on
  (goto _label_2))

(event `CardLocation`
  (params (Location :type "Vector Structure") (BoardSize :type Integer))
  (bind _boardsize_x (`self.BoardSize_X`))
  (bind _tilesize (`self.TileSize`))
  (bind _boardindex (`self.BoardIndex`))
  (bind _returnvalue (/ _tilesize 2.0))
  ;[1 1 1] Animation of putting cards on table, and removing them
  (set `self.CardLocationOffset` Location)
  (set `self.BoardSize_X` BoardSize)
  (bind (_direction _spawn) (`Timeline|PutCardOnDesk` :!via `PlayFromStart`)
    (:`Update`
      (`self.K2_SetActorLocation` (`KismetMathLibrary.VLerp` (`self.K2_GetActorLocation` (`self.Deck`)) (`KismetMathLibrary.MakeVector` (- (+ (+ (* (`KismetMathLibrary.Conv_IntToDouble` (mod _boardindex _boardsize_x)) _tilesize) _returnvalue) 34.8) (.x (`self.CardLocationOffset`))) (- (+ (+ (* (`KismetMathLibrary.Conv_IntToDouble` (/ _boardindex _boardsize_x)) _tilesize) _returnvalue) 22.4) (.y (`self.CardLocationOffset`))) (`self.VerticalOffset`)) _spawn))
      (`self.SetActorRelativeScale3D` (0.05 0.05 0.05)))
    (:`Finished`
      (set `self.BlockClick` false))))

(event `RotateCard`
  ;[1 1 1] Card rotation
  (`|ExecutionSequence`
    (:`then_0`
      (`/Engine/EditorBlueprintResources/StandardMacros.Gate` false :!label _label_3
        (:`Exit`
          (`|ExecutionSequence`
            (:`then_0`
              (goto _label_3 :!via `Close`))
            (:`then_1`
              (set `self.BlockClick` true)
              (`|ExecutionSequence`
                (:`then_0`
                  (`GameplayStatics.PlaySoundAtLocation` "/Game/Assets/Sounds/CardFlip_Stereo_Cue.CardFlip_Stereo_cue" :!label _label_4) ; Sound CardFlip
                )
                (:`then_1`
                  (`ActorComponent.Activate` (`self.Rotate1`) true))
                (:`then_2`
                  (bind (_direction _angle _move) (`Timeline|Card Rotate` :!via `PlayFromStart` :!label _label_5)
                    (:`Update`
                      (`SceneComponent.K2_SetRelativeTransform` (`self.CardPicture`) (`KismetMathLibrary.MakeTransform` (`KismetMathLibrary.VLerp` (0.0 0.0 0.0) (0.0 0.0 3.2) _move) (`KismetMathLibrary.RLerp` (struct) (struct :`Pitch` 180.0) _angle) (0.8 0.8 1.0)) false false))
                    (:`Finished`
                      (`KismetSystemLibrary.Delay` 1.6)
                      (set `self.BlockClick` false))))))))))
    (:`then_1`
      (goto _label_6 :!via `Open`))))

(event `HideTheCards`
  (bind _boardsize_x (`self.BoardSize_X`))
  (bind _tilesize (`self.TileSize`))
  (bind _boardindex (`self.BoardIndex`))
  (bind _returnvalue (/ _tilesize 2.0))
  ;[1 1 1] Animation of putting cards on table, and removing them
  (bind (_direction _spawn) (`Timeline|HideCard` :!via `Reverse`)
    (:`Update`
      (`self.K2_SetActorLocation` (`KismetMathLibrary.VLerp` (`self.K2_GetActorLocation` (`self.Deck`)) (`KismetMathLibrary.MakeVector` (- (+ (+ (* (`KismetMathLibrary.Conv_IntToDouble` (mod _boardindex _boardsize_x)) _tilesize) _returnvalue) 34.8) (.x (`self.CardLocationOffset`))) (- (+ (+ (* (`KismetMathLibrary.Conv_IntToDouble` (/ _boardindex _boardsize_x)) _tilesize) _returnvalue) 22.4) (.y (`self.CardLocationOffset`))) (`self.VerticalOffset`)) _spawn)))
    (:`Finished`
      (`self.K2_DestroyActor`))))

(event `UnRotateCard`
  ;[1 1 1] Card rotation
  (`|ExecutionSequence`
    (:`then_0`
      (`/Engine/EditorBlueprintResources/StandardMacros.Gate` true :!label _label_6
        (:`Exit`
          (`|ExecutionSequence`
            (:`then_0`
              (goto _label_6 :!via `Close`))
            (:`then_1`
              (`|ExecutionSequence`
                (:`then_0`
                  (goto _label_4))
                (:`then_1`
                  (`ActorComponent.Activate` (`self.Rotate2`) true)
                  (`KismetSystemLibrary.Delay` 0.3)
                  (`ActorComponent.Activate` (`self.Dust`) true))
                (:`then_2`
                  (goto _label_5 :!via `ReverseFromEnd`))))))))
    (:`then_1`
      (goto _label_3 :!via `Open`))))

(fn `SetCardPicture`
  (params (CardType :type Integer))
  (bind _cardpicture (`self.CardPicture`))
  ;[1 1 1] Define Card picture
  (set `self.CardIType` CardType)
  (switch `int` (`self.CardIType`)
    (:`0`
      (`PrimitiveComponent.SetMaterial` _cardpicture 1 "/Game/Assets/Materials/T_Animal_01_D_Mat.T_Animal_01_D_Mat"))
    (:`1`
      (`PrimitiveComponent.SetMaterial` _cardpicture 1 "/Game/Assets/Materials/T_Animal_02_D_Mat.T_Animal_02_D_Mat"))
    (:`2`
      (`PrimitiveComponent.SetMaterial` _cardpicture 1 "/Game/Assets/Materials/T_Animal_03_D_Mat.T_Animal_03_D_Mat"))
    (:`3`
      (`PrimitiveComponent.SetMaterial` _cardpicture 1 "/Game/Assets/Materials/T_Animal_04_D_Mat.T_Animal_04_D_Mat"))
    (:`4`
      (`PrimitiveComponent.SetMaterial` _cardpicture 1 "/Game/Assets/Materials/T_Animal_05_D_Mat.T_Animal_05_D_Mat"))
    (:`5`
      (`PrimitiveComponent.SetMaterial` _cardpicture 1 "/Game/Assets/Materials/T_Animal_06_D_Mat.T_Animal_06_D_Mat"))
    (:`6`
      (`PrimitiveComponent.SetMaterial` _cardpicture 1 "/Game/Assets/Materials/T_Animal_07_D_Mat.T_Animal_07_D_Mat"))
    (:`7`
      (`PrimitiveComponent.SetMaterial` _cardpicture 1 "/Game/Assets/Materials/T_Animal_08_D_Mat.T_Animal_08_D_Mat"))
    (:`8`
      (`PrimitiveComponent.SetMaterial` _cardpicture 1 "/Game/Assets/Materials/T_Animal_09_D_Mat.T_Animal_09_D_Mat"))
    (:`9`
      (`PrimitiveComponent.SetMaterial` _cardpicture 1 "/Game/Assets/Materials/T_Animal_10_D_Mat.T_Animal_10_D_Mat"))
    (:`10`
      (`PrimitiveComponent.SetMaterial` _cardpicture 1 "/Game/Assets/Materials/M_Animal_11_D_Mat.M_Animal_11_D_Mat"))))

(fn `UserConstructionScript`
  ;[1 1 1] Initial on card spawn
  (`self.SetCardPicture` (`self.CardIType`)))